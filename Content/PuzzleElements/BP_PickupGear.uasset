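; BP_PickupGear is a puzzle gear actor that BP_MotionController can pick up and drop.
; Pickup disables mesh physics and attaches the root to the given component, keeping world transform, while Drop re-enables physics and detaches.
; Each tick, RotateIndirection adds a world-space roll of RotationValue to the mesh while ShouldRotate is true, with no delta-time scaling.
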(event `/Game/VirtualRealityBP/Blueprints/PickupActorInterface.Pickup`
  (params (AttachTo :type "SceneComponent Object Reference"))
  (`PrimitiveComponent.SetSimulatePhysics` (`self.StaticMeshComponent`) false)
  (`SceneComponent.K2_AttachToComponent` (`self.K2_GetRootComponent`) AttachTo "None" "KeepWorld" "KeepWorld" "KeepWorld" false))

(event `self.ReceiveTick`
  (params (DeltaSeconds :type "Float (single-precision)"))
  (`self.RotateIndirection` (`self.ShouldRotate`)))

(event `/Game/VirtualRealityBP/Blueprints/PickupActorInterface.Drop`
  (`PrimitiveComponent.SetSimulatePhysics` (`self.StaticMeshComponent`) true)
  (`self.K2_DetachFromActor` "KeepWorld" "KeepWorld" "KeepWorld"))

(fn `RotateIndirection`
  (params (ShouldRotate :type Boolean))
  (if ShouldRotate
    (`SceneComponent.K2_AddWorldRotation` (`self.StaticMeshComponent`) (`KismetMathLibrary.MakeRotator` (`self.RotationValue`)) false false)))

(fn `UserConstructionScript`)